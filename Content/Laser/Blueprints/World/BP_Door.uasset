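; Level exit door that slides open when activated and ends the game with a victory screen when the player enters its trigger.
; ActivationStatus drives a Timeline that moves the Cube along local Y, opening only while CanOpen is set and reversing on deactivation.
; The player's first Box overlap locks and closes the door, disables input and shows WBP_FinalScreen with UI-only input and cursor.
; Any other actor overlapping the Box is destroyed.
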(event OnComponentBeginOverlap(Box)
  (params (OverlappedComponent :type Primitive%20Component%20Object%20Reference) (OtherActor :type Actor%20Object%20Reference) (OtherComp :type Primitive%20Component%20Object%20Reference) (OtherBodyIndex :type Integer) (bFromSweep :type Boolean) (SweepResult :type Hit%20Result%20Structure%20%28by%20ref%29))
  (bind _returnvalue (Game|GetPlayerController 0))
  (if (== OtherActor (Game|GetPlayerCharacter 0))
    (Utilities|FlowControl|DoOnce false
      (:Completed
        (Variables|Default|SetbCanOpen false)
        (CallFunction|CloseDoor)
        ;[0.5 0 0.5] Победный экран
        (Input|DisableInput (Game|GetPlayerCharacter 0) _returnvalue)
        (bind _returnvalue_2 (UserInterface|CreateWidget "/Game/Laser/Blueprints/World/Widgets/WBP_FinalScreen.WBP_FinalScreen_C" _returnvalue))
        (UserInterface|Viewport|AddtoViewport _returnvalue_2 0)
        (Input|SetInputModeUIOnly _returnvalue _returnvalue_2 "DoNotLock" false)
        (Variables|/Script/Engine.PlayerController|SetbShowMouseCursor _returnvalue true)))
    (else
      (Actor|DestroyActor OtherActor))))

(event Custom|CloseDoor
  (bind _newtrack_0 (Timeline|Timeline Reverse)
    (:Update
      (Transformation|SetRelativeLocation (Variables|Default|GetCube) (Math|Vector|MakeVector 0.0 (* _newtrack_0 -2e+02) 0.0) false false))))

(event EventBeginPlay)

(event Collision|EventActorBeginOverlap
  (params (OtherActor :type Actor%20Object%20Reference)))

(event EventTick
  (params (DeltaSeconds :type Float%20%28single-precision%29)))

(event EventActivationStatus
  (params (bNewStatus :type Boolean))
  (if bNewStatus
    (if (Variables|Default|GetbCanOpen)
      (bind _newtrack_0 (Timeline|Timeline Play)
        (:Update
          (Transformation|SetRelativeLocation (Variables|Default|GetCube) (Math|Vector|MakeVector 0.0 (* _newtrack_0 -2e+02) 0.0) false false))))
    (else
      (Timeline|Timeline Reverse))))

(fn ConstructionScript)