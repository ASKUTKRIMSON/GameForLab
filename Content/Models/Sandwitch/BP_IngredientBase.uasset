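; BP_IngredientBase is a base sandwich ingredient Actor, with early logic for cutting and stacking.
; On a mesh hit with another ingredient, an unstuck ingredient moves to its own SnapPoint, runs an attach call, disables the other's physics and shows W_VictoryScreen.
; It then marks itself stuck and increments an attachment count, printing completion at three.
; RegisterCut only counts cuts, and TryAttachIngredient is an empty stub.
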(event OnComponentHit(StaticMesh)
  (params (HitComponent :type Primitive%20Component%20Object%20Reference) (OtherActor :type Actor%20Object%20Reference) (OtherComp :type Primitive%20Component%20Object%20Reference) (NormalImpulse :type Vector :default "0, 0, 0") (Hit :type Hit%20Result%20Structure%20%28by%20ref%29))
  (bind _asbp_ingredient_base (Utilities|Casting|CastToBP_IngredientBase OtherActor))
  (if (not (Variables|Default|GetbIsStuck))
    (bind _output_get (Variables|Default|SetParentIngredient _asbp_ingredient_base))
    (Transformation|SetActorLocation (Transformation|GetWorldLocation (Variables|Default|GetSnapPoint)) false false)
    (Transformation|AttachComponentToComponent _output_get (Variables|BP_IngredientBase_C|GetStaticMesh (Variables|Default|GetParentIngredient)) "None" "KeepRelative" "KeepRelative" "KeepRelative" false)
    (Variables|Default|SetbIsStuck false)
    (Physics|SetSimulatePhysics (Variables|BP_IngredientBase_C|GetStaticMesh _output_get) false)
    (bind _returnvalue (UserInterface|CreateWidget "/Game/Models/UI/W_VictoryScreen.W_VictoryScreen_C"))
    (UserInterface|Viewport|AddtoViewport _returnvalue 0)
    (Variables|Default|SetbIsStuck true)
    (Variables|Default|SetAttachedIngredientsCount (+ (Variables|Default|GetAttachedIngredientsCount) 1))
    (if (>= (Variables|Default|GetAttachedIngredientsCount) 3)
      (Development|PrintString "Sandwitch is complete"))))

(event Custom|RegisterCut
  (if (Variables|Knife|GetCuttable)
    (Math|Integer|IncrementInt (Variables|Knife|GetCutCount)
      (:%20%20
        (if (>= (Variables|Knife|GetCutCount) (Variables|Knife|GetMaxCuts))
          _)))))

(event Collision|EventActorBeginOverlap
  (params (OtherActor :type Actor%20Object%20Reference)))

(event EventBeginPlay)

(fn ConstructionScript)

(fn TryAttachIngredient)